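; Red cube Blueprint that the player can use once close, switching off its collision and triggering an attached MovingCubeBP to move.
; Every Tick, while collision is enabled, it tints the mesh's tileColor material parameter from red to white as player distance grows between configurable min and max.
; Once collision is disabled through SetCollisionActivation, Tick paints the mesh flat grey instead.
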(event `self.ReceiveTick`
  (params (DeltaSeconds :type "Float (single-precision)"))
  (bind _staticmeshcomponent (`self.StaticMeshComponent`))
  (if (`self.IsCollisionEnabled`)
    (`MeshComponent.SetVectorParameterValueOnMaterials` _staticmeshcomponent "tileColor" (`KismetMathLibrary.Conv_LinearColorToVector` (`KismetMathLibrary.LinearColorLerp` (`KismetMathLibrary.MakeColor` 0.724) (`KismetMathLibrary.MakeColor` 1.0 1.0 1.0) (`KismetMathLibrary.FClamp` (`KismetMathLibrary.NormalizeToRange` (`KismetMathLibrary.Abs` (`KismetMathLibrary.VSize` (- (`SceneComponent.K2_GetComponentLocation` (`Actor.RootComponent` (`GameplayStatics.GetPlayerPawn` 0))) (`SceneComponent.K2_GetComponentLocation` (`self.StaticMeshComponent`))))) (`self.MinDistanceToPlayer`) (`self.MaxDistanceToPlayer`))))))
    (else
      (bind _returnvalue (`KismetMaterialLibrary.GetVectorParameterValue` null "titleColor"))
      (`MeshComponent.SetVectorParameterValueOnMaterials` _staticmeshcomponent "tileColor" (`KismetMathLibrary.Conv_LinearColorToVector` (`KismetMathLibrary.MakeColor` 0.5 0.5 0.5))))))

(fn `SetCollisionActivation`
  (params (`Activated?` :type Boolean))
  (bind _cube (`self.Cube`))
  (bind _output_get (set `self.IsCollisionEnabled` `Activated?`))
  (if _output_get
    (`PrimitiveComponent.SetCollisionEnabled` _cube "QueryAndPhysics")
    (else
      (`PrimitiveComponent.SetCollisionEnabled` _cube "NoCollision"))))

(fn `UsedByPlayer`
  (bind _attachedraiseobject (`self.AttachedRaiseObject`))
  (`self.SetCollisionActivation` false)
  (if (`KismetSystemLibrary.IsValid` _attachedraiseobject)
    (bind _asmoving_cube_bp (cast `/Game/MovingCubeBP` _attachedraiseobject))
    (`/Game/MovingCubeBP.DoMoveCube` _asmoving_cube_bp)))

(fn `UserConstructionScript`)