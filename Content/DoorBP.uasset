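; Door actor that opens once every blue cube in its ConnectedBlueCubes list is activated.
; Each Tick it scans the cubes and stops at the first inactive one.
; If none is inactive, which includes an empty list, it clears its IsActivated flag, disables mesh collision and zeroes the material Opacity parameter.
; No logic here closes the door again.
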(event `self.ReceiveTick`
  (params (DeltaSeconds :type "Float (single-precision)"))
  (bind _staticmeshcomponent (`self.StaticMeshComponent`))
  (set `self.WasABlueCubeNotActivated` false)
  (for _array_element (`self.ConnectedBlueCubes`)
    (if (not (`/Game/BlueCubeBP.IsActivated` _array_element))
      (set `self.WasABlueCubeNotActivated` true)
      (break)))
  (if (not (`self.WasABlueCubeNotActivated`))
    (set `self.IsActivated` false)
    (`PrimitiveComponent.SetCollisionEnabled` _staticmeshcomponent "NoCollision")
    (`MeshComponent.SetScalarParameterValueOnMaterials` _staticmeshcomponent "Opacity" 0.0)))

(fn `UserConstructionScript`)