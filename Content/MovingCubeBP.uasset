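; MovingCubeBP is an actor whose static mesh slides once from its starting position to an offset position when triggered.
; BeginPlay records the mesh's world location, and DoMoveCube sets a flag that starts the move.
; Tick then advances a clamped alpha by MoveSpeed and delta time, lerping the mesh toward the start plus MoveOffset without sweeping, with no reset or return.
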(event `self.ReceiveBeginPlay`
  ;[1 1 1] Begin
  (set `self.OriginalLocation` (`SceneComponent.K2_GetComponentLocation` (`self.StaticMeshComponent`))))

(event `self.ReceiveTick`
  (params (DeltaSeconds :type "Float (single-precision)"))
  (bind _originallocation (`self.OriginalLocation`))
  ;[1 1 1] Tick
  (if (and (`self.HasCubeMoved`) (< (`self.MoveAlpha`) 1.0))
    (bind _output_get (set `self.MoveAlpha` (`KismetMathLibrary.FClamp` (+ (* DeltaSeconds (`self.MoveSpeed`)) (`self.MoveAlpha`)))))
    (`SceneComponent.K2_SetWorldLocation` (`self.StaticMeshComponent`) (`KismetMathLibrary.VLerp` _originallocation (+ _originallocation (`self.MoveOffset`)) _output_get) false false)))

(fn `DoMoveCube`
  (set `self.HasCubeMoved` true))

(fn `UserConstructionScript`)