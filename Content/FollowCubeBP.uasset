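; FollowCubeBP is a floating, spinning companion cube that trails the player pawn's ball and visually "talks" when it plays sound clips.
; Tick lerps the mesh toward the ball plus follower offset with a sine bob.
; While audio plays, it samples the clip's amplitude at the tracked playback time to blend the material color toward TalkColor.
; When the pawn's DoEndStuff flag is set, looping timers flash the color and randomly flicker opacity.
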(event `OnAudioPlaybackPercent_Event`
  (params (PlayingSoundWave :type "SoundWave Object Reference") (PlaybackPercent :type "Float (double-precision)"))
  (set `self.CurrentSoundClipTime` (* PlaybackPercent (`SoundBase.Duration` PlayingSoundWave))))

(event `self.ReceiveBeginPlay`
  (add `AudioComponent.OnAudioPlaybackPercent` (`self.Audio`) (delegate `OnAudioPlaybackPercent_Event`))
  (bind _asplayer_pawn (cast `/Game/PlayerPawn` (`GameplayStatics.GetPlayerPawn` 0)))
  (set `self.PlayerPawn` _asplayer_pawn)
  (`KismetSystemLibrary.K2_SetTimer` null "ColorFlash" 0.6 true)
  (`KismetSystemLibrary.K2_SetTimer` null "OpacityFlash" (`KismetMathLibrary.RandomFloatInRange` 0.01 0.2) true))

(event `self.ReceiveTick`
  (params (DeltaSeconds :type "Float (single-precision)"))
  (bind _staticmeshcomponent (`self.StaticMeshComponent`))
  (bind _playerpawn (`self.PlayerPawn`))
  (bind _output_get (set `self.FloatyZSinCounter` (+ (* DeltaSeconds (`self.FloatyZSpeed`)) (`self.FloatyZSinCounter`))))
  (set `self.FloatyZOffset` (* (`KismetMathLibrary.Sin` _output_get) (`self.FloatyZAmount`)))
  (`SceneComponent.K2_SetWorldLocation` _staticmeshcomponent (`KismetMathLibrary.VLerp` (`SceneComponent.K2_GetComponentLocation` _staticmeshcomponent) (+ (`SceneComponent.K2_GetComponentLocation` (`/Game/PlayerPawn.Ball` _playerpawn)) (`/Game/PlayerPawn.FollowerPosition` _playerpawn) (`KismetMathLibrary.MakeVector` 0.0 0.0 (`self.FloatyZOffset`))) 0.1) false false)
  (`SceneComponent.K2_AddLocalRotation` (`self.StaticMeshComponent`) (`KismetMathLibrary.MakeRotator` 0.0 0.0 1.0) false false)
  (if (`AudioComponent.IsPlaying` (`self.Audio`))
    (bind _outamplitudes (`SoundVisualizationStatics.GetAmplitude` (`self.CurrentSoundClip`) 0 (`self.CurrentSoundClipTime`) 0.1 1))
    (for _array_element _outamplitudes
      (`MeshComponent.SetVectorParameterValueOnMaterials` (`self.StaticMeshComponent`) "Color" (`KismetMathLibrary.Conv_LinearColorToVector` (`KismetMathLibrary.LinearColorLerp` (`self.NormalColor`) (`self.TalkColor`) (/ _array_element 3000.0)))))))

(fn `ColorFlash`
  (bind _staticmeshcomponent (`self.StaticMeshComponent`))
  (if (`/Game/PlayerPawn.DoEndStuff` (`self.PlayerPawn`))
    (if (`self.ColorIsFlash`)
      (`MeshComponent.SetVectorParameterValueOnMaterials` _staticmeshcomponent "Color" (`KismetMathLibrary.Conv_LinearColorToVector` (`self.NormalColor`)))
      (set `self.ColorIsFlash` false)
      (else
        (`MeshComponent.SetVectorParameterValueOnMaterials` _staticmeshcomponent "Color" (`KismetMathLibrary.Conv_LinearColorToVector` (`self.FlashColor`)))
        (set `self.ColorIsFlash` true)))))

(fn `OpacityFlash`
  (if (`/Game/PlayerPawn.DoEndStuff` (`self.PlayerPawn`))
    (`MeshComponent.SetScalarParameterValueOnMaterials` (`self.StaticMeshComponent`) "Opacity" (`KismetMathLibrary.RandomFloatInRange` 0.6 1.0))
    (`KismetSystemLibrary.K2_SetTimer` null "OpacityFlash" (`KismetMathLibrary.RandomFloatInRange` 0.01 0.2) true)))

(fn `PlaySoundClip`
  (params (AudioClip :type "SoundWave Object Reference"))
  (bind _audio (`self.Audio`))
  (`AudioComponent.SetSound` _audio AudioClip)
  (`AudioComponent.Play` _audio 0.0)
  (set `self.CurrentSoundClip` AudioClip))

(fn `UserConstructionScript`)